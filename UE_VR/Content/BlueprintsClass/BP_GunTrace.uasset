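; BP_GunTrace is a hitscan gun that fires a line trace when its TriggerPressed event runs.
; A very long multi-object trace runs from the Arrow component along its forward vector against WorldDynamic and PhysicsBody objects, with persistent debug drawing.
; Every hit after the first that simulates physics receives an impulse scaled from the world-space impact point, rather than the shot direction.
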(event Collision|EventActorBeginOverlap
  (params (OtherActor :type Actor%20Object%20Reference))
  (|CallParentFunction OtherActor) ; This node is disabled and will not be called.\nDrag off pins to build functionality.
)

(event EventTick
  (params (DeltaSeconds :type Float%20%28single-precision%29))
  (|CallParentFunction DeltaSeconds) ; This node is disabled and will not be called.\nDrag off pins to build functionality.
)

(event EventTriggerPressed
  (bind _arrow (Variables|Default|GetArrow))
  (bind _returnvalue (Transformation|GetWorldLocation _arrow))
  (bind (_outhits _returnvalue_2) (Class|KismetSystemLibrary|LineTraceMultiforObjects _returnvalue (+ _returnvalue (* (Math|Vector|GetForwardVector _arrow) 999999.0)) (Utilities|Array|MakeArray "ObjectTypeQuery2" "ObjectTypeQuery4") true 0 "Persistent" true))
  (for (_array_element _array_index) _outhits
    (if _returnvalue_2
      (if (and (!= _array_index 0) (Physics|IsSimulatingPhysics (.HitComponent (Collision|BreakHitResult _array_element)) "None"))
        (Physics|AddImpulse (.HitComponent (Collision|BreakHitResult _array_element)) (* (.ImpactPoint (Collision|BreakHitResult _array_element)) 1e+02) "None" false)))))

(fn ConstructionScript
  (|CallParentFunction))