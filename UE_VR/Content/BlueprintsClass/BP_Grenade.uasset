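; BP_Grenade is a grenade actor that explodes on a delay after its trigger is released.
; TriggerReleased starts a one-shot five-second timer bound to the Explode event.
; Explode spawns the P_Explosion emitter, scaled up, at the static mesh's world location, then destroys the actor.
; The explosion is purely visual, as the graph applies no damage or physics force.
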(event Custom|Explode
  (Effects|SpawnEmitteratLocation "/Game/StarterContent/Particles/P_Explosion.P_Explosion" (Transformation|GetWorldLocation (Variables|Default|GetStaticMesh)) "0, 0, 0" "2.000000,2.000000,3.000000")
  (Actor|DestroyActor))

(event EventBeginPlay
  (|CallParentFunction) ; This node is disabled and will not be called.\nDrag off pins to build functionality.
)

(event Collision|EventActorBeginOverlap
  (params (OtherActor :type Actor%20Object%20Reference))
  (|CallParentFunction OtherActor) ; This node is disabled and will not be called.\nDrag off pins to build functionality.
)

(event EventTick
  (params (DeltaSeconds :type Float%20%28single-precision%29))
  (|CallParentFunction DeltaSeconds) ; This node is disabled and will not be called.\nDrag off pins to build functionality.
)

(event EventTriggerReleased
  (Utilities|Time|SetTimerbyEvent (delegate Custom|Explode) 5.0))

(fn ConstructionScript
  (|CallParentFunction))