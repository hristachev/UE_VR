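; BP_LaserSword is a toggleable laser sword that cuts procedural meshes it touches.
; ActionButton flip-flops the blade on and off by changing the Laser's Z scale and material and HiddenBlade's visibility.
; While on, Laser overlaps slice the mesh along HiddenBlade's plane, cap the cut with emissive material and enable physics on the new half.
; A DoOnce, reset on end overlap, prevents repeated slicing.
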(event OnComponentBeginOverlap(Laser)
  (params (OverlappedComponent :type Primitive%20Component%20Object%20Reference) (OtherActor :type Actor%20Object%20Reference) (OtherComp :type Primitive%20Component%20Object%20Reference) (OtherBodyIndex :type Integer) (bFromSweep :type Boolean) (SweepResult :type Hit%20Result%20Structure%20%28by%20ref%29))
  (bind _hiddenblade (Variables|Default|GetHiddenBlade))
  (Utilities|FlowControl|DoOnce false
    (:Completed
      (if (Variables|Default|GetBlade%20Visibility)
        (bind _asprocedural_mesh_component (Utilities|Casting|CastToProceduralMeshComponent OtherComp))
        (bind _outotherhalfprocmesh (Class|KismetProceduralMeshLibrary|SliceProceduralMesh _asprocedural_mesh_component (Transformation|GetWorldLocation _hiddenblade) (Math|Vector|GetUpVector _hiddenblade) true "CreateNewSectionForCap" "/Game/MyAssets/Materials/M_EmissiveBase_Inst.M_EmissiveBase_Inst"))
        (Physics|SetSimulatePhysics _outotherhalfprocmesh true)))))

(event OnComponentEndOverlap(Laser)
  (params (OverlappedComponent :type Primitive%20Component%20Object%20Reference) (OtherActor :type Actor%20Object%20Reference) (OtherComp :type Primitive%20Component%20Object%20Reference) (OtherBodyIndex :type Integer))
  (bind _hiddenblade (Variables|Default|GetHiddenBlade))
  (Utilities|FlowControl|DoOnce false) ; enters at Reset
)

(event EventBeginPlay
  (|CallParentFunction) ; This node is disabled and will not be called.\nDrag off pins to build functionality.
)

(event Collision|EventActorBeginOverlap
  (params (OtherActor :type Actor%20Object%20Reference))
  (|CallParentFunction OtherActor) ; This node is disabled and will not be called.\nDrag off pins to build functionality.
)

(event EventTick
  (params (DeltaSeconds :type Float%20%28single-precision%29))
  (|CallParentFunction DeltaSeconds) ; This node is disabled and will not be called.\nDrag off pins to build functionality.
)

(event EventActionButton
  (bind _laser (Variables|Default|GetLaser))
  (bind _returnvalue (Transformation|GetWorldScale _laser))
  (Utilities|FlowControl|FlipFlop
    (:A
      (Transformation|SetWorldScale3D _laser (Math|Vector|MakeVector (.x _returnvalue) (.y _returnvalue) 0.75))
      (Rendering|Material|SetMaterial (Variables|Default|GetLaser) 0 "/Game/MyAssets/Materials/M_EmissiveBase_Inst.M_EmissiveBase_Inst")
      (Rendering|SetVisibility (Variables|Default|GetHiddenBlade) true false)
      (Variables|Default|SetBlade%20Visibility true))
    (:B
      (Transformation|SetWorldScale3D _laser (Math|Vector|MakeVector (.x _returnvalue) (.y _returnvalue) 0.0))
      (Rendering|Material|SetMaterial (Variables|Default|GetLaser) 0 "/Game/StarterContent/Materials/M_Basic_Wall.M_Basic_Wall")
      (Rendering|SetVisibility (Variables|Default|GetHiddenBlade) false false)
      (Variables|Default|SetBlade%20Visibility false))))

(fn ConstructionScript
  (|CallParentFunction))