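; BP_Door is a door that swings open on its yaw axis when activated.
; Activate calls Iteract, which checks IsOpen, sets the timeline play rate from TimeToOpen or TimeToClose, then calls Open or Close.
; Open plays the OpenDoor timeline, lerping the mesh yaw from ClosePosition to OpenPosition and flipping IsOpen when finished.
; Close only stops the timeline, so it neither swings the door back nor clears IsOpen.
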(event Custom|Close
  (bind _door_track (Timeline|OpenDoor Stop)
    (:Update
      (Transformation|SetRelativeRotation (Variables|Default|GetStaticMesh) (Math|Rotator|MakeRotator 0.0 0.0 (Math|Float|Lerp (Variables|Default|GetClose%20Position) (Variables|Default|GetOpen%20Position) _door_track)) false false))
    (:Finished
      (Variables|Default|SetIsOpen (not (Variables|Default|GetIsOpen))))))

(event Custom|Open
  (bind _door_track (Timeline|OpenDoor Play)
    (:Update
      (Transformation|SetRelativeRotation (Variables|Default|GetStaticMesh) (Math|Rotator|MakeRotator 0.0 0.0 (Math|Float|Lerp (Variables|Default|GetClose%20Position) (Variables|Default|GetOpen%20Position) _door_track)) false false))
    (:Finished
      (Variables|Default|SetIsOpen (not (Variables|Default|GetIsOpen))))))

(event EventBeginPlay)

(event Collision|EventActorBeginOverlap
  (params (OtherActor :type Actor%20Object%20Reference)))

(event EventTick
  (params (DeltaSeconds :type Float%20%28single-precision%29)))

(event EventActivate
  (CallFunction|Iteract))

(fn ConstructionScript)

(fn Iteract
  (bind _opendoor (Variables|Default|GetOpenDoor))
  (if (not (Variables|Default|GetIsOpen))
    (Components|Timeline|SetPlayRate _opendoor (/ 1.0 (Variables|Default|GetTime%20To%20Open)))
    (CallFunction|Open)
    (else
      (Components|Timeline|SetPlayRate _opendoor (/ 1.0 (Variables|Default|GetTime%20To%20Close)))
      (CallFunction|Close)))
  (return))