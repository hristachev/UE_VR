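; BP_InventorySlot is an inventory slot that tracks an overlapping inventory item and can grab it.
; Its sphere overlap stores the latest BP_InventoryItemClass actor to enter and clears it when that same actor leaves.
; The Put event, if the stored item is valid, calls TryGrab on the item's GrabComponent with a MotionController reference.
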(event OnComponentBeginOverlap(Sphere)
  (params (OverlappedComponent :type Primitive%20Component%20Object%20Reference) (OtherActor :type Actor%20Object%20Reference) (OtherComp :type Primitive%20Component%20Object%20Reference) (OtherBodyIndex :type Integer) (bFromSweep :type Boolean) (SweepResult :type Hit%20Result%20Structure%20%28by%20ref%29))
  (bind _asbp_inventory_item_class (Utilities|Casting|CastToBP_InventoryItemClass OtherActor))
  (Variables|Default|SetAs%20BP%20Inventory%20Item%20Class _asbp_inventory_item_class))

(event OnComponentEndOverlap(Sphere)
  (params (OverlappedComponent :type Primitive%20Component%20Object%20Reference) (OtherActor :type Actor%20Object%20Reference) (OtherComp :type Primitive%20Component%20Object%20Reference) (OtherBodyIndex :type Integer))
  (bind _asbp_inventory_item_class (Utilities|Casting|CastToBP_InventoryItemClass OtherActor))
  (if (== _asbp_inventory_item_class (Variables|Default|GetAs%20BP%20Inventory%20Item%20Class))
    (Variables|Default|SetAs%20BP%20Inventory%20Item%20Class 0)))

(event Custom|Put
  (bind _as_bp_inventory_item_class (Variables|Default|GetAs%20BP%20Inventory%20Item%20Class))
  (Utilities|IsValid _as_bp_inventory_item_class
    (:Is%20Valid
      (Default|TryGrab (Variables|/Game/BlueprintsClass/BaseClass/BP_VRGrabClass.BP_VRGrabClass_C|GetGrabComponent _as_bp_inventory_item_class) (Variables|Default|GetMotionController)))))

(event EventBeginPlay)

(event Collision|EventActorBeginOverlap
  (params (OtherActor :type Actor%20Object%20Reference)))

(event EventTick
  (params (DeltaSeconds :type Float%20%28single-precision%29)))

(fn ConstructionScript)