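; Player pawn with motion-controller interaction: yaw-relative movement, controller look, teleporting and right-hand grabbing.
; Pushing the left stick runs a looping timer that projects an arc from the right controller onto the navmesh; release moves the pawn to any valid point.
; Grab checks the hand sphere's last overlapping actor for VRInteractionBPI, then calls its GrabComponent.
; Four smaller right-hand spheres set per-finger overlap flags.
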(event OnComponentBeginOverlap(SphereRightHand1)
  (params (OverlappedComponent :type Primitive%20Component%20Object%20Reference) (OtherActor :type Actor%20Object%20Reference) (OtherComp :type Primitive%20Component%20Object%20Reference) (OtherBodyIndex :type Integer) (bFromSweep :type Boolean) (SweepResult :type Hit%20Result%20Structure%20%28by%20ref%29))
  (Variables|Default|SetThump true))

(event OnComponentEndOverlap(SphereRightHand1)
  (params (OverlappedComponent :type Primitive%20Component%20Object%20Reference) (OtherActor :type Actor%20Object%20Reference) (OtherComp :type Primitive%20Component%20Object%20Reference) (OtherBodyIndex :type Integer))
  (Variables|Default|SetThump false))

(event OnComponentBeginOverlap(SphereRightHand2)
  (params (OverlappedComponent :type Primitive%20Component%20Object%20Reference) (OtherActor :type Actor%20Object%20Reference) (OtherComp :type Primitive%20Component%20Object%20Reference) (OtherBodyIndex :type Integer) (bFromSweep :type Boolean) (SweepResult :type Hit%20Result%20Structure%20%28by%20ref%29))
  (Variables|Default|SetIndex true))

(event OnComponentEndOverlap(SphereRightHand2)
  (params (OverlappedComponent :type Primitive%20Component%20Object%20Reference) (OtherActor :type Actor%20Object%20Reference) (OtherComp :type Primitive%20Component%20Object%20Reference) (OtherBodyIndex :type Integer))
  (Variables|Default|SetIndex false))

(event OnComponentBeginOverlap(SphereRightHand3)
  (params (OverlappedComponent :type Primitive%20Component%20Object%20Reference) (OtherActor :type Actor%20Object%20Reference) (OtherComp :type Primitive%20Component%20Object%20Reference) (OtherBodyIndex :type Integer) (bFromSweep :type Boolean) (SweepResult :type Hit%20Result%20Structure%20%28by%20ref%29))
  (Variables|Default|SetMiddle true))

(event OnComponentEndOverlap(SphereRightHand3)
  (params (OverlappedComponent :type Primitive%20Component%20Object%20Reference) (OtherActor :type Actor%20Object%20Reference) (OtherComp :type Primitive%20Component%20Object%20Reference) (OtherBodyIndex :type Integer))
  (Variables|Default|SetMiddle false))

(event OnComponentBeginOverlap(SphereRightHand4)
  (params (OverlappedComponent :type Primitive%20Component%20Object%20Reference) (OtherActor :type Actor%20Object%20Reference) (OtherComp :type Primitive%20Component%20Object%20Reference) (OtherBodyIndex :type Integer) (bFromSweep :type Boolean) (SweepResult :type Hit%20Result%20Structure%20%28by%20ref%29))
  (Variables|Default|SetRing true))

(event OnComponentEndOverlap(SphereRightHand4)
  (params (OverlappedComponent :type Primitive%20Component%20Object%20Reference) (OtherActor :type Actor%20Object%20Reference) (OtherComp :type Primitive%20Component%20Object%20Reference) (OtherBodyIndex :type Integer))
  (Variables|Default|SetRing false))

(event Input|ActionEvents|InputActionGrabRight
  (params (Key :type Key%20Structure :default "None"))
  (:Pressed
    (bind _actor (CallFunction|TryGrip (Variables|Default|GetSphereRightHand)))
    (Utilities|IsValid _actor
      (:Is%20Valid
        (bind _output_get (Variables|Default|SetActor%20Right (.AsBP%20VRGrab%20Class (Utilities|Casting|CastToBP_VRGrabClass _actor))))
        (Default|TryGrab (Variables|/Game/BlueprintsClass/BaseClass/BP_VRGrabClass.BP_VRGrabClass_C|GetGrabComponent _output_get) (Variables|Default|GetMotionControllerRight)))))
  (:Released
    (Utilities|IsValid (Variables|Default|GetActor%20Right)
      (:Is%20Valid
        (Default|TryRelease (Variables|/Game/BlueprintsClass/BaseClass/BP_VRGrabClass.BP_VRGrabClass_C|GetGrabComponent (Variables|Default|GetActor%20Right)))))))

(event Input|AxisEvents|InputAxisMovementAxisLeft_Y
  (params (AxisValue :type Float%20%28single-precision%29))
  (if (>= AxisValue 0.8)
    (CallFunction|ActivateTeleport)
    (else
      (CallFunction|DeactivateTeleport))))

(event Input|AxisEvents|InputAxisMovementAxisRight_X
  (params (AxisValue :type Float%20%28single-precision%29))
  (Pawn|Input|AddMovementInput (Math|Vector|GetForwardVector (Math|Rotator|MakeRotator 0.0 0.0 (.Yaw (Math|Rotator|BreakRotator (Pawn|GetControlRotation :!class /Script/Engine.Pawn))))) AxisValue false))

(event Input|AxisEvents|InputAxisMovementAxisRight_Y
  (params (AxisValue :type Float%20%28single-precision%29))
  (Pawn|Input|AddMovementInput (Math|Vector|GetRightVector (Math|Rotator|MakeRotator 0.0 0.0 (.Yaw (Math|Rotator|BreakRotator (Pawn|GetControlRotation :!class /Script/Engine.Pawn))))) AxisValue false))

(event Input|AxisEvents|InputAxisSpectatorYaw
  (params (AxisValue :type Float%20%28single-precision%29))
  (Pawn|Input|AddControllerYawInput AxisValue))

(event Input|AxisEvents|InputAxisSpectatorPitch
  (params (AxisValue :type Float%20%28single-precision%29))
  (Pawn|Input|AddControllerPitchInput AxisValue))

(event Input|AxisEvents|InputAxisGrabAxisRight
  (params (AxisValue :type Float%20%28single-precision%29))
  (Variables|Default|SetGrabRight AxisValue))

(fn ConstructionScript)

(fn DeactivateTeleport
  (if (Utilities|Time|IsValidTimerHandle (Variables|Default|GetTeleportHandleTimer))
    (Utilities|Time|ClearandInvalidateTimerbyHandle (Variables|Default|GetTeleportHandleTimer))
    (Variables|Default|SetTeleportHandleTimer "")
    (Variables|Default|SetIsTeleportActive? false)
    (Rendering|SetVisibility (Variables|Default|GetTeleport) false true)
    (if (Variables|Default|GetCanTeleport)
      (Transformation|SetActorLocation (+ (Transformation|GetWorldLocation (Variables|Default|GetTeleport)) "0,0,80.000000") false false))))

(fn UpdateTraceTeleport
  (bind _motioncontrollerright (Variables|Default|GetMotionControllerRight))
  (bind _teleport (Variables|Default|GetTeleport))
  (bind _outhit (Class|GameplayStatics|BlueprintPredictProjectilePathbyObjectType (Transformation|GetWorldLocation _motioncontrollerright) (* (Math|Vector|GetForwardVector _motioncontrollerright) 5e+03) true 1e+01 (Utilities|Array|MakeArray "ObjectTypeQuery1") false 0 "None"))
  (Rendering|SetVisibility _teleport (.ReturnValue (AI|Navigation|ProjectPointtoNavigation (Class|NavigationSystemV1|GetNavigationSystem) (.Location (Collision|BreakHitResult _outhit)) 0 0)) true)
  (Transformation|SetWorldLocation _teleport (.ProjectedLocation (AI|Navigation|ProjectPointtoNavigation (Class|NavigationSystemV1|GetNavigationSystem) (.Location (Collision|BreakHitResult _outhit)) 0 0)) false false)
  (Variables|Default|SetCanTeleport (.ReturnValue (AI|Navigation|ProjectPointtoNavigation (Class|NavigationSystemV1|GetNavigationSystem) (.Location (Collision|BreakHitResult _outhit)) 0 0))))

(fn ActivateTeleport
  (if (not (Variables|Default|GetIsTeleportActive?))
    (Variables|Default|SetIsTeleportActive? true)
    (Rendering|SetVisibility (Variables|Default|GetTeleport) true true)
    (bind _returnvalue (Utilities|Time|SetTimerbyFunctionName 0 "UpdateTraceTeleport" 0.1 true))
    (Variables|Default|SetTeleportHandleTimer _returnvalue)))

(fn TryDrop)

(fn TryGrip
  (params (Sphere :type Primitive%20Component%20Object%20Reference))
  (bind _overlappingactors (Collision|GetOverlappingActors Sphere 0 :!class /Script/Engine.PrimitiveComponent))
  (bind _returnvalue (Utilities|Array|LastIndex _overlappingactors))
  (bind _output (Utilities|Array|Get(acopy) _overlappingactors _returnvalue))
  (if (Utilities|DoesObjectImplementInterface _output "/Game/VRTemplate/Blueprints/VRInteractionBPI.VRInteractionBPI_C")
    (return _output)))